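; BP_PawnTank is a tank pawn that shows a player action grid widget during its turn.
; On turn start it calls the parent logic, waits briefly, creates WBP_PlayerActionGrid for its player controller and places it beside the pawn's projected screen position.
; The position is set once rather than tracked, and debug strings report progress.
; On turn end it removes the widget and restores game-only input.
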(event EventOnTurnStarted
  (|CallParentFunction)
  (Utilities|FlowControl|Delay 0.2)
  (bind _as플레이어_컨트롤러 (Utilities|Casting|CastToPlayerController (Pawn|GetController))
    (:then
      (Development|PrintString "Cast Succeeded")
      (bind _returnvalue (UserInterface|CreateWidget "/Game/BluePrints/Widgets/WBP_PlayerActionGrid.WBP_PlayerActionGrid_C" _as플레이어_컨트롤러))
      (Development|PrintString "Create Widget Succeeded")
      (bind _output_get (Variables|Default|SetActionWidgetReference _returnvalue))
      (UserInterface|Viewport|AddtoViewport _output_get 0)
      (if (.ReturnValue (Class|GameplayStatics|ProjectWorldtoScreen _as플레이어_컨트롤러 (Transformation|GetActorLocation) false))
        (Class|UserWidget|SetPositioninViewport (Variables|Default|GetActionWidgetReference) (+ (.ScreenPosition (Class|GameplayStatics|ProjectWorldtoScreen _as플레이어_컨트롤러 (Transformation|GetActorLocation) false)) "(X=100.000000,Y=-100.000000)") true)))
    (:CastFailed
      (Development|PrintString "CAST FAILED"))))

(event EventOnTurnEnded
  (Widget|RemovefromParent (Variables|Default|GetActionWidgetReference))
  (bind _as플레이어_컨트롤러 (Utilities|Casting|CastToPlayerController (Pawn|GetController)))
  (Input|SetInputModeGameOnly _as플레이어_컨트롤러 false))

(fn ConstructionScript)